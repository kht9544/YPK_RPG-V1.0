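; Knight player Blueprint that sets up the look of the character's mesh and sword Niagara effect.
; The construction script applies MainColor to both the Niagara color and the mesh's EmissiveColor_01 material parameter.
; It also passes storm rate and storm and smoke gravity to the effect; RateSmoke is written to User.RateStom and immediately overwritten by RateStom.
; The event graph holds only empty placeholder events.
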(fn `UserConstructionScript`
  (`NiagaraComponent.SetNiagaraVariableLinearColor` (`self.Niagara_Sward`) "User.MainColor" (`self.MainColor`))
  (`MeshComponent.SetVectorParameterValueOnMaterials` (`self.Mesh`) "EmissiveColor_01" (`KismetMathLibrary.Conv_LinearColorToVector` (`self.MainColor`)))
  (`NiagaraComponent.SetVariableFloat` (`self.Niagara_Sward`) "User.RateStom" (`self.RateSmoke`))
  (`NiagaraComponent.SetVariableFloat` (`self.Niagara_Sward`) "User.RateStom" (`self.RateStom`))
  (`NiagaraComponent.SetVariableVec3` (`self.Niagara_Sward`) "User.GravityStom" (`self.GravityStom`))
  (`NiagaraComponent.SetVariableVec3` (`self.Niagara_Sward`) "User.GravitySmoke" (`self.GravitySmoke`)))