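; Base monster Blueprint that plays a dissolve effect when the monster dies.
; MonsterIsDead creates dynamic material instances for the body mesh, shield and weapon, sharing a dissolve texture with the PDissolveEdge Niagara effect.
; A timeline drives Amount from one to zero on materials and particles together, then zeroes the Niagara Width when finished.
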(event `self.ReceiveTick`
  (params (DeltaSeconds :type "Float (single-precision)")))

(event `MonsterIsDead`
  (bind _mesh (`self.Mesh`))
  (bind _p_dissolveedge (`self.P_DissolveEdge`))
  (bind _texture (`self.Texture`))
  ;[1 1 1] 캐릭터 스켈레탈메쉬가 들고있는 Material 0, 1, 2
  (bind _returnvalue (`PrimitiveComponent.CreateDynamicMaterialInstance` _mesh 0 "/Game/SKnight_modular/Skeleton/materials/MI_Skeleton_Inst.MI_Skeleton_Inst" "None"))
  (bind _returnvalue_2 (`PrimitiveComponent.CreateDynamicMaterialInstance` _mesh 1 "/Game/SKnight_modular/Skeleton_Knight_01/materials/MatInst/MI_SKnigh_01_armor_Inst.MI_SKnigh_01_armor_Inst" "None"))
  (bind _returnvalue_3 (`PrimitiveComponent.CreateDynamicMaterialInstance` _mesh 2 "/Game/SKnight_modular/Skeleton_Knight_01/materials/MatInst/MI_SKnigh_01_armor_Inst.MI_SKnigh_01_armor_Inst" "None"))
  ;[1 1 1] 스켈레탈메쉬 검, 방패
  (bind _returnvalue_4 (`PrimitiveComponent.CreateDynamicMaterialInstance` (`self.sk_shield`) 0 "/Game/SKnight_modular/Skeleton_Knight_01/materials/MatInst/MI_Shield_01_Inst_Inst.MI_Shield_01_Inst_Inst" "None"))
  (bind _returnvalue_5 (`PrimitiveComponent.CreateDynamicMaterialInstance` (`self.sk_weapon`) 0 "/Game/SKnight_modular/Skeleton_Knight_01/materials/MatInst/MI_weapon_01_Inst.MI_weapon_01_Inst" "None"))
  (`MaterialInstanceDynamic.SetTextureParameterValue` _returnvalue "Texture" _texture)
  (`MaterialInstanceDynamic.SetTextureParameterValue` _returnvalue_2 "Texture" _texture)
  (`MaterialInstanceDynamic.SetTextureParameterValue` _returnvalue_3 "Texture" _texture)
  (`MaterialInstanceDynamic.SetTextureParameterValue` _returnvalue_4 "Texture" _texture)
  (`MaterialInstanceDynamic.SetTextureParameterValue` _returnvalue_5 "Texture" _texture)
  (`NiagaraFunctionLibrary.SetTextureObject` (`self.P_DissolveEdge`) "Texture" _texture)
  (bind (_direction `_새_트랙_0`) (`Timeline|타임라인` :!via `PlayFromStart`)
    (:`Update`
      (`MaterialInstanceDynamic.SetScalarParameterValue` _returnvalue "Amount" (`KismetMathLibrary.Lerp` 1.0 0.0 `_새_트랙_0`))
      (`MaterialInstanceDynamic.SetScalarParameterValue` _returnvalue_5 "Amount" (`KismetMathLibrary.Lerp` 1.0 0.0 `_새_트랙_0`))
      (`MaterialInstanceDynamic.SetScalarParameterValue` _returnvalue_4 "Amount" (`KismetMathLibrary.Lerp` 1.0 0.0 `_새_트랙_0`))
      (`MaterialInstanceDynamic.SetScalarParameterValue` _returnvalue_3 "Amount" (`KismetMathLibrary.Lerp` 1.0 0.0 `_새_트랙_0`))
      (`MaterialInstanceDynamic.SetScalarParameterValue` _returnvalue_2 "Amount" (`KismetMathLibrary.Lerp` 1.0 0.0 `_새_트랙_0`))
      (`NiagaraComponent.SetVariableFloat` _p_dissolveedge "User.Amount" (`KismetMathLibrary.Lerp` 1.0 0.0 `_새_트랙_0`)))
    (:`Finished`
      (`NiagaraComponent.SetVariableFloat` _p_dissolveedge "User.Width" 0.0))))

(fn `UserConstructionScript`)